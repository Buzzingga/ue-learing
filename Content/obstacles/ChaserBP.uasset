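; Chaser obstacle character that pursues the player inside a trigger radius and knocks them away on contact.
; Entering the chase sphere opens a gate that re-issues an AI move to the player's location on a short delay loop; leaving closes it.
; Overlapping the player launches them along the flattened direction away from the chaser with upward lift and plays a smash sound.
; The construction script applies configurable radius and walk speed.
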(event OnComponentBeginOverlap(overlap)
  (params (OverlappedComponent :type Primitive%20Component%20Object%20Reference) (OtherActor :type Actor%20Object%20Reference) (OtherComp :type Primitive%20Component%20Object%20Reference) (OtherBodyIndex :type Integer) (bFromSweep :type Boolean) (SweepResult :type Hit%20Result%20Structure%20%28by%20ref%29))
  ;[1 1 1] launch
  (bind _astpc_link (Utilities|Casting|CastToTPC_Link OtherActor))
  (Character|LaunchCharacter _astpc_link (* (Math|Vector|MakeVector (.x (Math|Vector|Normalize (Math|Vector|MakeVector (.x (Math|Vector|GetUnitDirection(Vector) (Transformation|GetWorldLocation (Variables|Collision|GetCapsuleComponent)) (Transformation|GetActorLocation _astpc_link))) (.y (Math|Vector|GetUnitDirection(Vector) (Transformation|GetWorldLocation (Variables|Collision|GetCapsuleComponent)) (Transformation|GetActorLocation _astpc_link))) 0.0))) (.y (Math|Vector|Normalize (Math|Vector|MakeVector (.x (Math|Vector|GetUnitDirection(Vector) (Transformation|GetWorldLocation (Variables|Collision|GetCapsuleComponent)) (Transformation|GetActorLocation _astpc_link))) (.y (Math|Vector|GetUnitDirection(Vector) (Transformation|GetWorldLocation (Variables|Collision|GetCapsuleComponent)) (Transformation|GetActorLocation _astpc_link))) 0.0))) 0.5) (Variables|Default|GetLaunch%20Velociy)) false false)
  (Audio|SpawnSoundatLocation "/Game/Sounds/smash_character.smash_character" (Transformation|GetActorLocation) "0, 0, 0" 1.0 0.2 0.0 0 0))

(event OnComponentBeginOverlap(ChaseRadius)
  (params (OverlappedComponent :type Primitive%20Component%20Object%20Reference) (OtherActor :type Actor%20Object%20Reference) (OtherComp :type Primitive%20Component%20Object%20Reference) (OtherBodyIndex :type Integer) (bFromSweep :type Boolean) (SweepResult :type Hit%20Result%20Structure%20%28by%20ref%29))
  (Utilities|Casting|CastToTPC_Link OtherActor)
  (CallFunction|ChasePlayer))

(event OnComponentEndOverlap(ChaseRadius)
  (params (OverlappedComponent :type Primitive%20Component%20Object%20Reference) (OtherActor :type Actor%20Object%20Reference) (OtherComp :type Primitive%20Component%20Object%20Reference) (OtherBodyIndex :type Integer))
  (Utilities|Casting|CastToTPC_Link OtherActor)
  (CallFunction|StopChasing))

(event Custom|ChasePlayer
  (Utilities|FlowControl|Sequence
    (:then_0
      (goto _label Open))
    (:then_1
      (Utilities|FlowControl|Gate true :!label _label
        (:Exit
          (AI|AIMoveTo self (Transformation|GetActorLocation (Game|GetPlayerCharacter 0)) 0 5.0 false
            (:then
              (Utilities|FlowControl|Delay 0.2)
              (goto _label))))))))

(event Custom|StopChasing
  (Utilities|FlowControl|Gate true) ; enters at Close
)

(fn ConstructionScript
  (Components|Sphere|SetSphereRadius (Variables|Default|GetChaseRadius) (Variables|Default|GetChase%20Trigger%20Rad) true)
  (Variables|/Script/Engine.CharacterMovementComponent|SetMaxWalkSpeed (Variables|Character|GetCharacterMovement) (Variables|Default|GetMoveSpeed)))