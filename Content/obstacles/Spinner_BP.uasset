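; Spinning pillar obstacle that knocks the TPC_Link character away and halts while a CryonisCubeBP overlaps its capsule.
; A timeline rotates the pivot at SpinRate, stopping and resuming as the cube enters and leaves.
; Character overlaps trigger an outward, upward launch with a smash sound, debounced by a briefly delayed DoOnce reset.
; The construction script scales and offsets the pillar and sizes the capsule from PillarScale.
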(event OnComponentBeginOverlap(Capsule)
  (params (OverlappedComponent :type Primitive%20Component%20Object%20Reference) (OtherActor :type Actor%20Object%20Reference) (OtherComp :type Primitive%20Component%20Object%20Reference) (OtherBodyIndex :type Integer) (bFromSweep :type Boolean) (SweepResult :type Hit%20Result%20Structure%20%28by%20ref%29))
  (Utilities|FlowControl|Sequence
    (:then_0
      (bind _astpc_link (Utilities|Casting|CastToTPC_Link OtherActor))
      (Utilities|FlowControl|DoOnce false :!label _label
        (:Completed
          (Utilities|FlowControl|Sequence
            (:then_0
              (CallFunction|LaunchCharacter _astpc_link _astpc_link))
            (:then_1
              (Utilities|FlowControl|Delay 0.2)
              (goto _label Reset))))))
    (:then_1
      (Utilities|Casting|CastToCryonisCubeBP OtherActor)
      (CallFunction|Stopspin))))

(event OnComponentEndOverlap(Capsule)
  (params (OverlappedComponent :type Primitive%20Component%20Object%20Reference) (OtherActor :type Actor%20Object%20Reference) (OtherComp :type Primitive%20Component%20Object%20Reference) (OtherBodyIndex :type Integer))
  (Utilities|Casting|CastToCryonisCubeBP OtherActor)
  (CallFunction|StartRotating))

(event Custom|StartRotating
  (Components|Timeline|SetPlayRate (Variables|Default|GetRotation) (Variables|Default|GetSpinRate))
  (bind _0_1 (Timeline|Rotation Play)
    (:Update
      (Transformation|SetRelativeRotation (Variables|Default|GetPivotScene) (Math|Rotator|Lerp(Rotator) "0, 0, 0" "0,360.000000, 0" _0_1) false false))))

(event Custom|Stopspin
  (bind _0_1 (Timeline|Rotation Stop)
    (:Update
      (Transformation|SetRelativeRotation (Variables|Default|GetPivotScene) (Math|Rotator|Lerp(Rotator) "0, 0, 0" "0,360.000000, 0" _0_1) false false))))

(event EventBeginPlay
  (CallFunction|StartRotating))

(fn ConstructionScript
  (bind _capsule (Variables|Default|GetCapsule))
  (Transformation|SetWorldScale3D (Variables|Default|GetPillar) (Variables|Default|GetPillar%20Scale))
  (Transformation|SetRelativeLocation (Variables|Default|GetPillar) (Math|Vector|MakeVector (* (/ (* (.z (Variables|Default|GetPillar%20Scale)) 1e+02) 2.0) -1.0) 0.0 0.0) false false)
  (Components|Capsule|SetCapsuleHalfHeight _capsule (+ (/ (* (.z (Variables|Default|GetPillar%20Scale)) 1e+02) 2.0) 5e+01) true)
  (Components|Capsule|SetCapsuleRadius _capsule (+ (/ (* (.x (Variables|Default|GetPillar%20Scale)) 1e+02) 2.0) 2e+01) true))

(fn LaunchCharacter
  (params (Character :type Character%20Object%20Reference) (Location :type Actor%20Object%20Reference))
  (bind _returnvalue (Transformation|GetActorLocation Location))
  (bind _defaultsceneroot (Variables|Default|GetDefaultSceneRoot))
  (bind _returnvalue_2 (Transformation|GetWorldLocation _defaultsceneroot))
  (bind _returnvalue_3 (Math|Vector|GetUnitDirection(Vector) _returnvalue_2 _returnvalue))
  (Character|LaunchCharacter Character (* (Math|Vector|Normalize (+ (Math|Vector|Normalize (Math|Vector|MakeVector (.x _returnvalue_3) (.y _returnvalue_3) 0.0)) "0, 0,1.000000")) (Variables|Default|GetLaunchSpeed)) false false)
  (Audio|SpawnSoundatLocation "/Game/Sounds/smash_character.smash_character" (Transformation|GetActorLocation) "0, 0, 0" 1.0 1.0 0.0 0 0))