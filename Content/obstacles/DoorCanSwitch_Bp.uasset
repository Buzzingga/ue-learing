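; Switch-unlocked double door obstacle that plays a locked sound when TPC_Link enters its overlap volume while locked.
; Binds to its Switch's button-pressed event, which clears IsLocked, opens the door and turns the lock light green.
; A timeline lerps both doors from their starting rotations to opposite yaws, with a DoOnce-gated opening sound.
; The construction script colors the lock light red or green from IsLocked.
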(event OnComponentBeginOverlap(Overlap)
  (params (OverlappedComponent :type Primitive%20Component%20Object%20Reference) (OtherActor :type Actor%20Object%20Reference) (OtherComp :type Primitive%20Component%20Object%20Reference) (OtherBodyIndex :type Integer) (bFromSweep :type Boolean) (SweepResult :type Hit%20Result%20Structure%20%28by%20ref%29))
  (Utilities|Casting|CastToTPC_Link OtherActor)
  (if (Variables|Default|GetIsLocked)
    (Audio|SpawnSound2D "/Game/Sounds/Door__is_locked.Door__is_locked" 1.0 1.0 0.0 0)))

(event Custom|OpenDoor
  (if (not (Variables|Default|GetIsLocked))
    (bind _0_1 (Timeline|0-1 Play)
      (:Update
        (Transformation|SetRelativeRotation (Variables|Default|GetDoor1) (Math|Rotator|Lerp(Rotator) (Variables|Default|GetDoor1Origin) "0,-90.000000, 0" _0_1 true) false false)
        (Transformation|SetRelativeRotation (Variables|Default|GetDoor2) (Math|Rotator|Lerp(Rotator) (Variables|Default|GetDoor2Orign) "0,90.000000, 0" _0_1 true) false false)
        (Utilities|FlowControl|DoOnce false
          (:Completed
            (Audio|SpawnSound2D "/Game/Sounds/Doors_open.Doors_open" 1.0 1.0 0.0 0)))))))

(event Custom|UnlockDoor
  (params (Button :type Button%20BP%20Object%20Reference))
  (if (== Button (Variables|Default|Getswitch))
    (bind _output_get (Variables|Default|SetIsLocked false))
    (CallFunction|OpenDoor)
    (if _output_get
      (Rendering|Components|Light|SetLightColor (Variables|Default|GetLocklight) "(R=1.000000,G=0.000000,B=0.025606,A=1.000000)" true)
      (else
        (Rendering|Components|Light|SetLightColor (Variables|Default|GetLocklight) "(R=0.430328,G=1.000000,B=0.066689,A=1.000000)" true)))))

(event EventBeginPlay
  (Variables|Default|SetDoor1Origin (Variables|/Script/Engine.SceneComponent|GetRelativeRotation (Variables|Default|GetDoor1)))
  (Variables|Default|SetDoor2Orign (Variables|/Script/Engine.SceneComponent|GetRelativeRotation (Variables|Default|GetDoor2)))
  (EventDispatchers|BindEventtoButtonPressed (Variables|Default|Getswitch) (delegate Custom|UnlockDoor)))

(fn ConstructionScript
  (if (Variables|Default|GetIsLocked)
    (Rendering|Components|Light|SetLightColor (Variables|Default|GetLocklight) "(R=1.000000,G=0.000000,B=0.025606,A=1.000000)" true)
    (else
      (Rendering|Components|Light|SetLightColor (Variables|Default|GetLocklight) "(R=0.430328,G=1.000000,B=0.066689,A=1.000000)" true))))