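; Moving platform obstacle that runs while its linked pressure button is pressed and halts when it is released.
; At BeginPlay it caches the relative locations of two position markers, scales the timeline rate by cycle time and binds to the button's pressed and unpressed events.
; The timeline lerps the platform between the markers without sweep, stopping in place and resuming from that point.
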(event Custom|StartMoving
  (bind _0_1 (Timeline|0-1 Play)
    (:Update
      (Transformation|SetRelativeLocation (Variables|Default|Getplatform) (Math|Vector|Lerp(Vector) (Variables|Default|GetMove1) (Variables|Default|GetMove2) _0_1) false false))))

(event Custom|StopMoving
  (bind _0_1 (Timeline|0-1 Stop)
    (:Update
      (Transformation|SetRelativeLocation (Variables|Default|Getplatform) (Math|Vector|Lerp(Vector) (Variables|Default|GetMove1) (Variables|Default|GetMove2) _0_1) false false))))

(event Custom|UnLock
  (params (Button :type Button%20Platform%20Can%20Reactive%20BP%20Object%20Reference))
  (if (== Button (Variables|Default|GetButtonPlat))
    (CallFunction|StartMoving)))

(event Custom|Lock
  (params (ButtonPlat :type Button%20Platform%20Can%20Reactive%20BP%20Object%20Reference))
  (if (== ButtonPlat (Variables|Default|GetButtonPlat))
    (CallFunction|StopMoving)))

(event EventBeginPlay
  (Variables|Default|SetMove1 (Variables|/Script/Engine.SceneComponent|GetRelativeLocation (Variables|Default|GetMovePos1)))
  (Variables|Default|SetMove2 (Variables|/Script/Engine.SceneComponent|GetRelativeLocation (Variables|Default|GetMovePos2)))
  (Components|Timeline|SetPlayRate (Variables|Default|Get0-1) (/ 1.0 (Variables|Default|GetCycleTime)))
  (EventDispatchers|BindEventtoButtonPlatPressed (Variables|Default|GetButtonPlat) (delegate Custom|UnLock))
  (EventDispatchers|BindEventtoButtonPlatUnPressed (Variables|Default|GetButtonPlat) (delegate Custom|Lock)))

(fn ConstructionScript)