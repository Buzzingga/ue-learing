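; Moving platform obstacle that starts moving when its linked one-time button is pressed.
; On BeginPlay it caches two marker component positions, scales a timeline's play rate from CycleTime, and binds to the button's pressed event.
; The button press plays a confirmation sound and runs the timeline, which lerps the platform's relative location between the two points.
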(event Custom|StartMoving
  (bind _0_1 (Timeline|0-1 Play)
    (:Update
      (Transformation|SetRelativeLocation (Variables|Default|Getplatform) (Math|Vector|Lerp(Vector) (Variables|Default|GetMove1) (Variables|Default|GetMove2) _0_1) false false))))

(event Custom|Unlock
  (params (ButtonOnce :type Button%20Platform%20Once%20BP%20Object%20Reference))
  (if (== ButtonOnce (Variables|Default|GetButtonOnce))
    (Audio|SpawnSound2D "/Game/Sounds/Correct.Correct" 1.0 1.0 0.0 0)
    (CallFunction|StartMoving)))

(event EventBeginPlay
  (Variables|Default|SetMove1 (Variables|/Script/Engine.SceneComponent|GetRelativeLocation (Variables|Default|GetMovePos1)))
  (Variables|Default|SetMove2 (Variables|/Script/Engine.SceneComponent|GetRelativeLocation (Variables|Default|GetMovePos2)))
  (Components|Timeline|SetPlayRate (Variables|Default|Get0-1) (/ 1.0 (Variables|Default|GetCycleTime)))
  (EventDispatchers|BindEventtoButtonPlatPressed (Variables|Default|GetButtonOnce) (delegate Custom|Unlock)))

(fn ConstructionScript)