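; AutoFloorBP is an obstacle-folder Blueprint that procedurally builds a grid of instanced meshes, named as an automatic floor.
; The construction script applies the Material variable to slot 0 of the InstancedStaticMesh, then nested loops over Numx and Numy add evenly spaced instances.
; The grid spans the component's local X and Z axes, with Y fixed at zero.
; The event graph holds only disabled placeholder events, so it adds no runtime logic.
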(event EventBeginPlay)

(event Collision|EventActorBeginOverlap
  (params (OtherActor :type Actor%20Object%20Reference)))

(event EventTick
  (params (DeltaSeconds :type Float%20%28single-precision%29)))

(fn ConstructionScript
  (Rendering|Material|SetMaterial (Variables|Default|GetInstancedStaticMesh) 0 (Variables|Default|GetMaterial))
  (for _index (range 0 (- (Variables|Default|GetNumx) 1))
    (LocalVariables|SetLOOPX _index)
    (for _index_2 (range 0 (- (Variables|Default|GetNumy) 1))
      (LocalVariables|SetLOOPY _index_2)
      (Components|InstancedStaticMesh|AddInstance (Variables|Default|GetInstancedStaticMesh) (Math|Transform|MakeTransform (Math|Vector|MakeVector (* (LocalVariables|GetLOOPX) 5e+02) 0.0 (* (LocalVariables|GetLOOPY) 5e+02)))))))