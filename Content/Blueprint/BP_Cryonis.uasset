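; Cryonis pillar actor that grows and retracts vertically, starting its expansion on BeginPlay.
; The Retractexpand timeline lerps Scene Z scale from nearly flat toward MaxHeight times PilarHeight, flagging it damageable and placeable.
; Expand plays or resets the preview, or stops looping once placed, while Destroy reverses the timeline and destroys the actor when finished.
; Box overlaps with anything except the player or BP_water only print debug strings.
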(event OnComponentBeginOverlap(Box)
  (params (OverlappedComponent :type Primitive%20Component%20Object%20Reference) (OtherActor :type Actor%20Object%20Reference) (OtherComp :type Primitive%20Component%20Object%20Reference) (OtherBodyIndex :type Integer) (bFromSweep :type Boolean) (SweepResult :type Hit%20Result%20Structure%20%28by%20ref%29))
  ;[1 1 1] overlap something then stop animation
  (if (and (!= OtherActor (Game|GetPlayerCharacter 0)) (!= (Utilities|GetClass OtherActor) "/Game/Blueprint/BP_water.BP_water_C"))
    (Development|PrintString "overlap")))

(event OnComponentEndOverlap(Box)
  (params (OverlappedComponent :type Primitive%20Component%20Object%20Reference) (OtherActor :type Actor%20Object%20Reference) (OtherComp :type Primitive%20Component%20Object%20Reference) (OtherBodyIndex :type Integer))
  ;[1 1 1] Endoverlap something then stop animation
  (if (and (!= OtherActor (Game|GetPlayerCharacter 0)) (!= (Utilities|GetClass OtherActor) "/Game/Blueprint/BP_water.BP_water_C"))
    (Development|PrintString "endoverlap")))

(event Custom|Expand
  (params (Expand :type Boolean) (PilarHeight :type Float%20%28single-precision%29))
  (Development|PrintString (Utilities|String|ToString(Float) PilarHeight) true true "(R=0.000000,G=0.660000,B=1.000000,A=1.000000)" 1.0)
  (if (not (Variables|Default|Getisplaced))
    (if Expand
      (bind (_direction _lerp) (Timeline|Retract/expand Play)
        (:Update
          ;[1 1 1] Set Croynis Scale
          (Transformation|SetRelativeScale3D (Variables|Default|GetScene) (Math|Vector|MakeVector 1.5 1.5 (Math|Float|Lerp 0.02 (* (Variables|Default|GetMaxHeight) PilarHeight) _lerp)))
          (Variables|Actor|SetbCanBeDamaged true)
          (Variables|Default|SetCanBePalced true))
        (:Finished
          ;[1 1 1] Destory Croynis
          (switch Utilities|FlowControl|Switch|SwitchonETimelineDirection _direction
            (:Backward
              (Actor|DestroyActor)))))
      (else
        ;[1 1 1] Stop Animation
        (Utilities|FlowControl|Sequence
          (:then_0
            (Timeline|Retract/expand Stop))
          (:then_1
            (Transformation|SetRelativeScale3D (Variables|Default|GetScene) (Math|Vector|MakeVector 1.5 1.5 0.02))
            (Variables|Default|SetCanBePalced false)))))
    (else
      ;[1 1 1] Stop Lopping
      (Components|Timeline|SetLooping (Variables|Default|GetRetract/expand) false)
      (Timeline|Retract/expand Play))))

(event Custom|Destroy
  ;[1 1 1] Destory Croynis
  (bind (_direction _lerp) (Timeline|Retract/expand ReverseFromEnd)
    (:Update
      ;[1 1 1] Set Croynis Scale
      (Transformation|SetRelativeScale3D (Variables|Default|GetScene) (Math|Vector|MakeVector 1.5 1.5 (Math|Float|Lerp 0.02 (* (Variables|Default|GetMaxHeight) (stale Custom|Expand PilarHeight)) _lerp)))
      (Variables|Actor|SetbCanBeDamaged true)
      (Variables|Default|SetCanBePalced true))
    (:Finished
      (switch Utilities|FlowControl|Switch|SwitchonETimelineDirection _direction
        (:Backward
          (Actor|DestroyActor))))))

(event Collision|EventActorBeginOverlap
  (params (OtherActor :type Actor%20Object%20Reference)))

(event EventTick
  (params (DeltaSeconds :type Float%20%28single-precision%29)))

(event EventBeginPlay
  (CallFunction|Expand true 1.0))

(fn ConstructionScript)