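; Fall-volume trigger that handles the player or puzzle objects dropping out of bounds, using an overlap box sized from a BoxExtent variable in the construction script.
; When TPC_Link enters, it plays a game-over sound, shows a FadetoBlack widget and reopens the current level after a short delay.
; Magnesis and stasis objects that enter instead receive their respective interaction messages.
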(event OnComponentBeginOverlap(overlap)
  (params (OverlappedComponent :type Primitive%20Component%20Object%20Reference) (OtherActor :type Actor%20Object%20Reference) (OtherComp :type Primitive%20Component%20Object%20Reference) (OtherBodyIndex :type Integer) (bFromSweep :type Boolean) (SweepResult :type Hit%20Result%20Structure%20%28by%20ref%29))
  (Utilities|FlowControl|Sequence
    (:then_0
      (Utilities|Casting|CastToTPC_Link OtherActor)
      (Audio|SpawnSound2D "/Game/Sounds/269190__mickleness__game-lose.269190__mickleness__game-lose" 1.0 1.0 0.0 0)
      (bind _returnvalue (UserInterface|CreateWidget "/Game/Check_point/FadetoBlack.FadetoBlack_C"))
      (Default|FadetoBlack _returnvalue)
      (UserInterface|Viewport|AddtoViewport _returnvalue 0)
      (Utilities|FlowControl|Delay 3.0)
      (bind _returnvalue_2 (Game|GetCurrentLevelName true))
      (Game|OpenLevel(byName) (Utilities|String|StringToName _returnvalue_2)))
    (:then_1
      (Utilities|Casting|CastToGenericMagnesisObject OtherActor)
      (Class|BPIItemMag|InteractionMag(Message) OtherActor))
    (:then_2
      (Utilities|Casting|CastToNewStasisObjectParent OtherActor)
      (Class|BPIItemMag|InteractionSta(Message) OtherActor)
      (Development|PrintString "detected"))))

(fn ConstructionScript
  (Components|Box|SetBoxExtent (Variables|Default|Getoverlap) (Variables|Default|GetBox%20Extent) true))