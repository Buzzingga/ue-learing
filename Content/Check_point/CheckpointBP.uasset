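; Checkpoint actor that saves the player's respawn transform when a TPC_Link character overlaps its trigger.
; On overlap it loads the CheckPointSaveGame slot, or creates a CheckpointSaveGame if none exists.
; It stores its own location raised along Z, with zero rotation, as the checkpoint and writes the slot.
; A Savegame_popup widget then shows a "Game Saved" notification.
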(event OnComponentBeginOverlap(overlap)
  (params (OverlappedComponent :type Primitive%20Component%20Object%20Reference) (OtherActor :type Actor%20Object%20Reference) (OtherComp :type Primitive%20Component%20Object%20Reference) (OtherBodyIndex :type Integer) (bFromSweep :type Boolean) (SweepResult :type Hit%20Result%20Structure%20%28by%20ref%29))
  (Utilities|Casting|CastToTPC_Link OtherActor)
  (bind _returnvalue (SaveGame|DoesSaveGameExist (Variables|Default|GetCheckPointSaveGame)))
  (if _returnvalue
    (bind _returnvalue_2 (SaveGame|LoadGamefromSlot (Variables|Default|GetCheckPointSaveGame)))
    (bind _ascheckpoint_save_game (Utilities|Casting|CastToCheckpointSaveGame _returnvalue_2))
    (Variables|Default|SetSave%20Game%20Reference _ascheckpoint_save_game)
    (else
      (bind _returnvalue_3 (SaveGame|CreateSaveGameObject "/Game/Check_point/CheckpointSaveGame.CheckpointSaveGame_C"))
      (Variables|Default|SetSave%20Game%20Reference _returnvalue_3)))
  (bind _output_get (Variables|/Game/Check_point/CheckpointSaveGame.CheckpointSaveGame_C|SetCheckpoint (Variables|Default|GetSave%20Game%20Reference) (Math|Transform|MakeTransform (+ (.location (Transformation|GetActorTransform)) "0, 0,200.000000"))))
  (SaveGame|SaveGametoSlot (Variables|Default|GetSave%20Game%20Reference) (Variables|Default|GetCheckPointSaveGame))
  (bind _returnvalue_4 (UserInterface|CreateWidget "/Game/Check_point/Savegame_popup.Savegame_popup_C"))
  (Default|DisplaySaveNodification _returnvalue_4 "Game Saved")
  (UserInterface|Viewport|AddtoViewport _returnvalue_4 0))

(fn ConstructionScript)