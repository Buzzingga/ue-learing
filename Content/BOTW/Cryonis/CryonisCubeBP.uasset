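; Ice pillar actor for a BOTW-style Cryonis ability, with a simulated mode and a rise animation.
; Construction sizes the pillar from a scale multiplier, applies a tinted dynamic ice material and caches the actor's bounds.
; Simulate mode disables collision and swaps in a glass material.
; ScaleUp runs a timeline at a configurable rate that lerps height from nearly flat to full size while keeping the footprint fixed.
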(event Custom|ScaleUp
  (bind _finalscale (Variables|Default|GetFinalScale))
  (bind (_x _y) (Math|Vector|BreakVector _finalscale))
  (Components|Timeline|SetPlayRate (Variables|Default|GetScale) (Variables|Default|GetScaleRate))
  (Transformation|SetWorldScale3D (Variables|Default|GetIcePillar) "1.000000,1.000000,0.010000")
  (bind _0_to_1 (Timeline|Scale Play)
    (:Update
      (Transformation|SetWorldScale3D (Variables|Default|GetIcePillar) (Math|Vector|Lerp(Vector) (Math|Vector|MakeVector _x _y 0.01) _finalscale _0_to_1)))))

(event Custom|SetPillarModeToSimulate
  (Collision|SetCollisionEnabled (Variables|Default|GetIcePillar) "NoCollision")
  (Rendering|Material|SetMaterial (Variables|Default|GetIcePillar) 0 "/Game/StarterContent/Materials/M_Glass.M_Glass"))

(event EventBeginPlay)

(fn ConstructionScript
  (bind _output_get (Variables|Default|SetFinalScale (* "0.800000,0.800000,1.200000" (Variables|Default|GetScaleTimes))))
  (Transformation|SetWorldScale3D (Variables|Default|GetIcePillar) _output_get)
  ;[1 1 1] Create mat
  (bind _returnvalue (Rendering|Material|CreateDynamicMaterialInstance (Variables|Default|GetIcePillar) 0 "/Game/BOTW/Cryonis/IceMat.IceMat" "None" :!class /Script/Engine.PrimitiveComponent))
  (bind _output_get_2 (Variables|Default|SetDynamicIceRef _returnvalue))
  (Rendering|Material|SetVectorParameterValue _output_get_2 "Color" (Variables|Default|GetIceBlue) :!class /Script/Engine.MaterialInstanceDynamic)
  (Variables|Default|SetPillarBounds (.BoxExtent (Collision|GetActorBounds false))))