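; ItemSpawner_BP spawns an ActorToSpawn instance at its own location and rotation on BeginPlay, with a configurable scale and itself as owner.
; The RespawnMag event clears CurrentItem, waits DelayBeforeRespawn, then attempts another spawn.
; AttemptToSpawn guards on CurrentItem, but SpawnItem sets it to None instead of storing the spawned actor.
; A random pick from ItemsToSpawn exists but is unused.
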(event EventBeginPlay
  (CallFunction|AttempttoSpawn))

(event EventRespawnMag
  (Variables|Default|SetCurrentItem 0)
  (Utilities|FlowControl|Delay (Variables|Default|GetDelayBeforeRespawn))
  (CallFunction|AttempttoSpawn))

(fn ConstructionScript)

(fn AttempttoSpawn
  (Utilities|IsValid (Variables|Default|GetCurrentItem)
    (:Is%20Valid
      (Development|PrintString "already spawned"))
    (:Is%20Not%20Valid
      (CallFunction|SpawnItem))))

(fn SpawnItem
  (Game|SpawnActorfromClass (Variables|Default|GetActorToSpawn) (Math|Transform|MakeTransform (Transformation|GetActorLocation) (Transformation|GetActorRotation) (Variables|Default|GetActorScale)) "Undefined" self 0)
  (Variables|Default|SetCurrentItem 0))