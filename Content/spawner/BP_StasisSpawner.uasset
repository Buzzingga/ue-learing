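; Spawner actor that places an instance of a configurable actor class at its own location and rotation, with a set scale.
; It attempts a spawn on BeginPlay, and its RespawnSta event clears CurrentItem, waits a configurable delay and tries again.
; The validity check on CurrentItem guards spawning, but Spawnitem sets that reference to None instead of storing the spawned actor, which it owns.
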(event EventBeginPlay
  (CallFunction|AttempttoSpawn))

(event EventRespawnSta
  (Variables|Default|SetCurrent%20item 0)
  (Utilities|FlowControl|Delay (Variables|Default|GetDelay%20Before%20Respawn))
  (CallFunction|AttempttoSpawn))

(fn ConstructionScript)

(fn AttempttoSpawn
  (Utilities|IsValid (Variables|Default|GetCurrent%20item)
    (:Is%20Not%20Valid
      (CallFunction|Spawnitem))))

(fn Spawnitem
  (Game|SpawnActorfromClass (Variables|Default|GetActorToSpawn) (Math|Transform|MakeTransform (Transformation|GetActorLocation) (Transformation|GetActorRotation) (Variables|Default|GetSpawnActorScale)) "Undefined" self 0)
  (Variables|Default|SetCurrent%20item 0))